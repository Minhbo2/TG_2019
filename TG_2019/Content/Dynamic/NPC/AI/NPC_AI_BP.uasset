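; AI controller for guard NPCs that runs the GuardBehavior behavior tree on the PatrolData blackboard.
; AI perception updates store a sensed actor in the Enemy key and clear it when sensing fails, ignoring actors tagged "Enemy" so AIs do not target each other.
; FindPatrolRoute casts the pawn to PatrollingGuard_BP2 and sets the WayPoint key with no value supplied; the event graph never calls it.
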(event `self.ReceiveBeginPlay`
  (bind _blackboardcomponent (`self.UseBlackboard` "/Game/Dynamic/NPC/AI/PatrolData.PatrolData"))
  (set `self.BBComp` _blackboardcomponent)
  (`self.RunBehaviorTree` "/Game/Dynamic/NPC/AI/GuardBehavior.GuardBehavior"))

(event `self.AIPerception.OnTargetPerceptionUpdated`
  (params (Actor :type "Actor Object Reference") (Stimulus :type "AIStimulus Structure"))
  (bind _enemy (`self.Enemy`))
  (bind _bbcomp (`self.BBComp`))
  ;[1 1 1] AI will not consider each other as Enemy
  (if (`self.ActorHasTag` Actor "Enemy")
    _
    (elif (`.bSuccessfullySensed` (break `AIStimulus` Stimulus))
      (`BlackboardComponent.SetValueAsObject` _bbcomp _enemy Actor)
      (else
        (`BlackboardComponent.ClearValue` _bbcomp _enemy)))))

(fn `FindPatrolRoute`
  (params (Blackboard :type "BlackboardComponent Object Reference"))
  (cast `/Game/Dynamic/NPC/Behaviors/PatrollingGuard_BP2` (`self.K2_GetPawn`))
  (`BlackboardComponent.SetValueAsObject` Blackboard "WayPoint" null))

(fn `UserConstructionScript`)