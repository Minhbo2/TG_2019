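; NPC AI controller that sets up the patrol blackboard and runs the guard behavior tree on BeginPlay.
; AI Perception updates write a sensed actor to the Enemy blackboard key and clear it when sensing fails, skipping actors tagged "Enemy" so AI ignore each other.
; A FindPatrolRoute function casts the pawn to Character_BP and sets the WayPoint key without a visible value, but nothing here calls it.
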(event `self.ReceiveBeginPlay`
  (bind _blackboardcomponent (`self.UseBlackboard` "/Game/Dynamic/Character/AI/PatrolData.PatrolData"))
  (set `self.BBComp` _blackboardcomponent)
  (`self.RunBehaviorTree` "/Game/Dynamic/Character/AI/GuardBehavior.GuardBehavior"))

(event `self.AIPerception.OnTargetPerceptionUpdated`
  (params (Actor :type "Actor Object Reference") (Stimulus :type "AIStimulus Structure"))
  (`self.UpdateBlackboard` Actor Stimulus Actor))

(fn `FindPatrolRoute`
  (params (Blackboard :type "BlackboardComponent Object Reference"))
  (cast `/Game/Dynamic/Character/Behaviors/Character_BP` (`self.K2_GetPawn`))
  (`BlackboardComponent.SetValueAsObject` Blackboard "WayPoint" null))

(fn `UpdateBlackboard`
  (params (`Self ` :type "Object Object Reference") (AIStimulus :type "AIStimulus Structure (by ref)") (`Other Actor` :type "Actor Object Reference"))
  (bind _enemy (`self.Enemy`))
  (bind _bbcomp (`self.BBComp`))
  ;[1 1 1] AI will not consider each other as Enemy, Add the tag on AI
  (if (`self.ActorHasTag` `Other Actor` "Enemy")
    _
    (elif (`.bSuccessfullySensed` (break `AIStimulus` AIStimulus))
      (`BlackboardComponent.SetValueAsObject` _bbcomp _enemy `Self `)
      (else
        (`BlackboardComponent.ClearValue` _bbcomp _enemy)))))

(fn `UserConstructionScript`)