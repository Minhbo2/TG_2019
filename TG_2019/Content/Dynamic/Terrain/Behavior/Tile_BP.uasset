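; Infinite-terrain tile that gates movement with a barrier and triggers spawning of further tiles.
; Entering the LockingVolume turns the barrier green and passable; leaving re-locks it red and asks InfiniteTerrain_GM to spawn a tile.
; Overlapping the DestroyVolume removes the tile, and GetAttachTransform exposes the AttachPoint transform.
; Overlaps are filtered by IsPlayerActor, which, despite its name, tests for the "Enemy" tag.
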(event `self.ReceiveBeginPlay`
  (`self.Locked`))

(event `self.LockingVolume.OnComponentBeginOverlap`
  (params (OverlappedComponent :type "PrimitiveComponent Object Reference") (OtherActor :type "Actor Object Reference") (OtherComp :type "PrimitiveComponent Object Reference") (OtherBodyIndex :type Integer) (bFromSweep :type Boolean) (SweepResult :type "HitResult Structure (by ref)"))
  (`self.IsPlayerActor` OtherActor
    (:`NewParam`
      (`self.Unlocked`))))

(event `self.LockingVolume.OnComponentEndOverlap`
  (params (OverlappedComponent :type "PrimitiveComponent Object Reference") (OtherActor :type "Actor Object Reference") (OtherComp :type "PrimitiveComponent Object Reference") (OtherBodyIndex :type Integer))
  (`self.IsPlayerActor` OtherActor
    (:`NewParam`
      (`self.Locked`)
      (bind _asinfinite_terrain_gm (cast `/Game/Dynamic/InfiniteTerrain_GM` (`GameplayStatics.GetGameMode`)))
      (`/Game/Dynamic/InfiniteTerrain_GM.SpawnTile` _asinfinite_terrain_gm))))

(event `self.DestroyVolume.OnComponentBeginOverlap`
  (params (OverlappedComponent :type "PrimitiveComponent Object Reference") (OtherActor :type "Actor Object Reference") (OtherComp :type "PrimitiveComponent Object Reference") (OtherBodyIndex :type Integer) (bFromSweep :type Boolean) (SweepResult :type "HitResult Structure (by ref)"))
  (`self.IsPlayerActor` OtherActor
    (:`NewParam`
      (`self.K2_DestroyActor`))))

(fn `GetAttachTransform`
  (returns (Location :type "Transform Structure"))
  (return (`SceneComponent.K2_GetComponentToWorld` (`self.AttachPoint`))))

(fn `Locked`
  (bind _barrier (`self.Barrier`))
  (`PrimitiveComponent.SetCollisionEnabled` _barrier "QueryAndPhysics")
  (`PrimitiveComponent.SetMaterial` _barrier 0 "/Game/Static/Geometry/Meshes/RedBarrier_M.RedBarrier_M"))

(fn `Unlocked`
  (bind _barrier (`self.Barrier`))
  (`PrimitiveComponent.SetCollisionEnabled` _barrier "NoCollision")
  (`PrimitiveComponent.SetMaterial` _barrier 0 "/Game/Static/Geometry/Meshes/GreenBarrier_M.GreenBarrier_M"))

(fn `UserConstructionScript`)